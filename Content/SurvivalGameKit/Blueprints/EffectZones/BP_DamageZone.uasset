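; BP_DamageZone is an effect volume that drains health from master characters standing inside it.
; Authority-only overlap events maintain a set of actors, unpausing a looping timer with an immediate first hit and pausing it once the set empties.
; Each tick deducts one health through each character's PlayerInventoryComponent, so DamagePerSec sets the tick frequency rather than the hit size.
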(event OnComponentBeginOverlap(DamageZone)
  (params (OverlappedComponent :type Primitive%20Component%20Object%20Reference) (OtherActor :type Actor%20Object%20Reference) (OtherComp :type Primitive%20Component%20Object%20Reference) (OtherBodyIndex :type Integer) (bFromSweep :type Boolean) (SweepResult :type Hit%20Result%20Structure%20%28by%20ref%29))
  ;[0 1 0.09084] Server events
  ;;[1 1 1] Actor begin overlap
  (|ActorBeginOverlap OtherActor))

(event OnComponentEndOverlap(DamageZone)
  (params (OverlappedComponent :type Primitive%20Component%20Object%20Reference) (OtherActor :type Actor%20Object%20Reference) (OtherComp :type Primitive%20Component%20Object%20Reference) (OtherBodyIndex :type Integer))
  ;[0 1 0.09084] Server events
  ;;[1 1 1] Actor end overlap
  (|ActorEndOverlap OtherActor))

(event EventBeginPlay
  ;[0 1 0.09084] Server events
  ;;[1 1 1] Begin play
  (|CreateDamageTimer))

(fn ConstructionScript)

(event Custom|Damage
  ;[1 1 1] Create damage timer
  ;;[1 1 1] Loop for all the actors in the volume
  (bind _result (Utilities|Set|ToArray (Variables|NonEdit|GetActors)))
  (for _array_element _result
    ;;[1 1 1] If the actor is a master character
    (bind _asbp_master_character (Utilities|Casting|CastToBP_MasterCharacter _array_element))
    (Utilities|IsValid (Variables|/Game/SurvivalGameKit/Blueprints/Characters/BP_MasterCharacter.BP_MasterCharacter_C|GetPlayerInventoryComponent _asbp_master_character)
      (:Is%20Valid
        ;;[1 1 1] Damage for 1 health
        (Default|DeductHealth (Variables|/Game/SurvivalGameKit/Blueprints/Characters/BP_MasterCharacter.BP_MasterCharacter_C|GetPlayerInventoryComponent _asbp_master_character) 1))
      (:Is%20Not%20Valid
        ;;[1 1 1] Remove actor from array
        (Utilities|Set|Remove (Variables|NonEdit|GetActors) _array_element)))))