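; BP_MasterResourceFoliageComponent is a foliage component in the survival kit that lets players interact with individual resource foliage instances.
; On Interact, if its Interactable is set, it asks the player component to server-replace the instance at the hit item index with that Interactable.
; The interaction query functions return mostly empty or false defaults, including IsInteractable; only the interacting action text reads a variable, InteractionTimerText.
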(event EventInteract
  (params (Player%20Component :type BP%20Player%20Inventory%20Component%20Object%20Reference))
  (bind _interactable (Variables|ResourceSettings|GetInteractable))
  (if _interactable
    (Default|ServerReplaceInstance Player%20Component self (.hititem (Variables|/Game/SurvivalGameKit/Blueprints/Components/BP_PlayerInventoryComponent.BP_PlayerInventoryComponent_C|GetServer%20Hit%20Result Player%20Component)) _interactable)))

(fn InteractAction
  (return ""))

(fn InteractInputBrush
  (return ""))

(fn InteractName
  (return ""))

(fn InteractTime
  (return false 0.0))

(fn InteractingActionText
  (return (Variables|ResourceSettings|GetInteraction%20Timer%20Text)))

(fn IsInteractable
  (return false))