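; Blueprint function library for the survival kit's inventory, providing shared lookups and checks on items, weapons and attachments.
; Detail functions find an item's ItemList row by ID and return the row, its attachment class, or its holdable class cast to master, ranged or melee weapon.
; Attachment checks require the weapon to allow the attachment and have that slot type empty.
; Other helpers find an item's cooking recipe by scanning CookingRecipes and compare inventory slots.
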(fn ItemDetails
  (params (Item%20In :type S%20Item%20Inventory%20Structure))
  ;[1 1 1] Get the items details
  (bind _returnvalue (Utilities|GetDataTableRow "/Game/SurvivalGameKit/Blueprints/Items/ItemList.ItemList" (Utilities|String|StringToName (.ID (Utilities|Struct|BreakS_ItemInventory Item%20In))))
    (:then
      (return true _returnvalue))
    (:RowNotFound
      (return false ""))))

(fn CheckAllowedAttachments
  (params (Attachment :type BP%20Master%20Attachment%20Class%20Reference) (Weapon :type BP%20Master%20Holdable%20Class%20Reference) (Weapon%20Attachments :type S%20Weapon%20Attachements%20Structure))
  ;[1 1 1] Set local variables
  (LocalVariables|SetAttachment%20L Attachment)
  (LocalVariables|SetWeapon%20L Weapon)
  (LocalVariables|SetWeapon%20Attachments%20L Weapon%20Attachments)
  ;[1 1 1] Cast to ranged weapon
  (bind _asbp_master_weapon (Utilities|Casting|CastToBP_MasterWeaponClass (LocalVariables|GetWeapon%20L))
    (:then
      ;[1 1 1] Is attachment allowed
      (if (Utilities|Set|Contains (.Allowed%20Attachments (Utilities|GetClassDefaults _asbp_master_weapon)) (LocalVariables|GetAttachment%20L))
        ;[1 1 1] Check if the weapon already has attachment in slot
        (if (Utilities|Enum|Equal(Enum) (.Attachment%20Type (Utilities|GetClassDefaults (LocalVariables|GetAttachment%20L))) "NewEnumerator0")
          (return (not (Utilities|IsValidClass (Utilities|Struct|BreakS_WeaponAttachements (LocalVariables|GetWeapon%20Attachments%20L)))))
          (elif (Utilities|Enum|Equal(Enum) (.Attachment%20Type (Utilities|GetClassDefaults (LocalVariables|GetAttachment%20L))) "NewEnumerator1")
            (return (not (Utilities|IsValidClass (Utilities|Struct|BreakS_WeaponAttachements (LocalVariables|GetWeapon%20Attachments%20L)))))
            (elif (Utilities|Enum|Equal(Enum) (.Attachment%20Type (Utilities|GetClassDefaults (LocalVariables|GetAttachment%20L))) "NewEnumerator2")
              (return (not (Utilities|IsValidClass (Utilities|Struct|BreakS_WeaponAttachements (LocalVariables|GetWeapon%20Attachments%20L)))))
              (elif (Utilities|Enum|Equal(Enum) (.Attachment%20Type (Utilities|GetClassDefaults (LocalVariables|GetAttachment%20L))) "NewEnumerator3")
                (return (not (Utilities|IsValidClass (Utilities|Struct|BreakS_WeaponAttachements (LocalVariables|GetWeapon%20Attachments%20L)))))
                (elif (Utilities|Enum|Equal(Enum) (.Attachment%20Type (Utilities|GetClassDefaults (LocalVariables|GetAttachment%20L))) "NewEnumerator4")
                  (return (not (Utilities|IsValidClass (Utilities|Struct|BreakS_WeaponAttachements (LocalVariables|GetWeapon%20Attachments%20L)))))
                  (elif (Utilities|Enum|Equal(Enum) (.Attachment%20Type (Utilities|GetClassDefaults (LocalVariables|GetAttachment%20L))) "NewEnumerator5")
                    (return (not (Utilities|IsValidClass (Utilities|Struct|BreakS_WeaponAttachements (LocalVariables|GetWeapon%20Attachments%20L)))))
                    (elif (Utilities|Enum|Equal(Enum) (.Attachment%20Type (Utilities|GetClassDefaults (LocalVariables|GetAttachment%20L))) "NewEnumerator6")
                      (return (not (Utilities|IsValidClass (Utilities|Struct|BreakS_WeaponAttachements (LocalVariables|GetWeapon%20Attachments%20L)))))
                      (elif (Utilities|Enum|Equal(Enum) (.Attachment%20Type (Utilities|GetClassDefaults (LocalVariables|GetAttachment%20L))) "NewEnumerator7")
                        (return (not (Utilities|IsValidClass (Utilities|Struct|BreakS_WeaponAttachements (LocalVariables|GetWeapon%20Attachments%20L)))))
                        (elif (Utilities|Enum|Equal(Enum) (.Attachment%20Type (Utilities|GetClassDefaults (LocalVariables|GetAttachment%20L))) "NewEnumerator8")
                          (return (not (Utilities|IsValidClass (Utilities|Struct|BreakS_WeaponAttachements (LocalVariables|GetWeapon%20Attachments%20L)))))
                          (else
                            (return false)))))))))))
        (else
          _)))
    (:CastFailed
      _))
  (return false))

(fn AttachmentDetails
  (params (Item :type S%20Item%20Inventory%20Structure))
  (bind _returnvalue (Utilities|GetDataTableRow "/Game/SurvivalGameKit/Blueprints/Items/ItemList.ItemList" (Utilities|String|StringToName (.ID (Utilities|Struct|BreakS_ItemInventory Item))))
    (:then
      (if (Utilities|IsValidClass (.AttachmentClass (Utilities|Struct|BreakS_ItemDetails _returnvalue)))
        (return true (.AttachmentClass (Utilities|Struct|BreakS_ItemDetails _returnvalue)))
        (else
          (return false 0))))))

(fn MasterWeaponDetails
  (params (Item :type S%20Item%20Inventory%20Structure))
  (bind _returnvalue (Utilities|GetDataTableRow "/Game/SurvivalGameKit/Blueprints/Items/ItemList.ItemList" (Utilities|String|StringToName (.ID (Utilities|Struct|BreakS_ItemInventory Item))))
    (:then
      (bind _asbp_master_weapon (Utilities|Casting|CastToBP_MasterWeaponClass (.HoldableClass (Utilities|Struct|BreakS_ItemDetails _returnvalue)))
        (:then
          (return true _asbp_master_weapon))
        (:CastFailed
          _)))
    (:RowNotFound
      _))
  (return false 0))

(fn RangeWeaponDetails
  (params (S_ItemInventory :type S%20Item%20Inventory%20Structure%20%28by%20ref%29))
  (bind _returnvalue (Utilities|GetDataTableRow "/Game/SurvivalGameKit/Blueprints/Items/ItemList.ItemList" (Utilities|String|StringToName (.ID (Utilities|Struct|BreakS_ItemInventory S_ItemInventory))))
    (:then
      (bind _asbp_master_range_weapon (Utilities|Casting|CastToBP_MasterRangeWeaponClass (.HoldableClass (Utilities|Struct|BreakS_ItemDetails _returnvalue)))
        (:then
          (return true _asbp_master_range_weapon))
        (:CastFailed
          _)))
    (:RowNotFound
      _))
  (return false 0))

(fn MeleeWeaponDetails
  (params (S_ItemInventory :type S%20Item%20Inventory%20Structure%20%28by%20ref%29))
  (bind _returnvalue (Utilities|GetDataTableRow "/Game/SurvivalGameKit/Blueprints/Items/ItemList.ItemList" (Utilities|String|StringToName (.ID (Utilities|Struct|BreakS_ItemInventory S_ItemInventory))))
    (:then
      (bind _asbp_master_melee_weapon (Utilities|Casting|CastToBP_MasterMeleeWeaponClass (.HoldableClass (Utilities|Struct|BreakS_ItemDetails _returnvalue)))
        (:then
          (return true _asbp_master_melee_weapon))
        (:CastFailed
          _)))
    (:RowNotFound
      _))
  (return false 0))

(fn ConvertData
  (params (Item :type S%20Item%20Inventory%20Structure))
  (LocalVariables|SetItem%20L Item)
  (bind _outrownames (DataTable|GetDataTableRowNames "/Game/SurvivalGameKit/Blueprints/Items/Recipes/CookingRecipes.CookingRecipes"))
  (for _array_element _outrownames
    (bind _returnvalue (Utilities|GetDataTableRow "/Game/SurvivalGameKit/Blueprints/Items/Recipes/CookingRecipes.CookingRecipes" _array_element)
      (:then
        (if (Utilities|Name|Equal(Name) (.RowName (Utilities|Struct|BreakDataTableRowHandle (.item (.StartItem (Utilities|Struct|BreakS_ConvertData _returnvalue))))) (Utilities|String|StringToName (.id (LocalVariables|GetItem%20L))))
          (return true _returnvalue)))))
  (return false ""))

(fn IsSameInventorySlot?
  (params (Item%201 :type S%20Item%20Inventory%20Structure) (Item%202 :type S%20Item%20Inventory%20Structure))
  (bind (_id _count _index _inventory) (Utilities|Struct|BreakS_ItemInventory Item%201))
  (bind (_id_2 _count_2 _index_2 _inventory_2) (Utilities|Struct|BreakS_ItemInventory Item%202))
  (if (and (== _index _index_2) (== _inventory_2 _inventory))
    (return true)
    (else
      (return false))))