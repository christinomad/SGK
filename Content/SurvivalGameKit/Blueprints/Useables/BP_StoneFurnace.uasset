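; BP_StoneFurnace is a useable stone furnace in the survival game kit that reacts visually and audibly to player targeting and interaction.
; Target and NotTarget events toggle custom depth on the furnace mesh.
; Interact animation events swap its material between normal and glowing variants while playing or stopping the fire sound, which is also stopped on BeginPlay.
; The construction script only calls the parent.
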(event EventBeginPlay
  ;[0 1 0.09084] Server events
  ;;[1 1 1] Begin play
  (Audio|Components|Audio|Stop (Variables|Default|GetFire%20Sound)))

(event EventTarget
  ;[0 0.5089 1] Client events
  ;;[1 1 1] Player target
  (Rendering|SetRenderCustomDepth (Variables|Default|GetFurnace) true))

(event EventNotTarget
  ;[0 0.5089 1] Client events
  ;;[1 1 1] Not a player target
  (Rendering|SetRenderCustomDepth (Variables|Default|GetFurnace) false))

(event EventSwitchOffInteractAnimation
  ;[0 1 0.09084] Server events
  ;;[1 1 1] Swich off animation
  (Rendering|Material|SetMaterial (Variables|Default|GetFurnace) 0 "/Game/SurvivalGameKit/Materials/M_Env_Fire_Furnace.M_Env_Fire_Furnace")
  (Audio|Components|Audio|Stop (Variables|Default|GetFire%20Sound)))

(event EventSwitchonInteractAnimation
  ;[0 1 0.09084] Server events
  ;;[1 1 1] Switch on interact animation
  (Rendering|Material|SetMaterial (Variables|Default|GetFurnace) 0 "/Game/SurvivalGameKit/Materials/M_Env_Fire_Furnace_glow.M_Env_Fire_Furnace_glow")
  (Audio|Components|Audio|Play (Variables|Default|GetFire%20Sound) 0.0))

(fn ConstructionScript
  (|CallParentFunction))