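; Stone furnace build part that players interact with through a convert inventory component, optionally restricted to listed owners.
; Targeting toggles custom depth on the furnace mesh, while switch on and off events swap between glowing and plain materials and start or stop the fire sound.
; Multicast destroy clears the mesh, shatters a destructible mesh when one is valid, then removes the actor after a delay, or immediately without one.
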(event EventBeginPlay
  ;[0 1 0.09084] Server events
  ;;[1 1 1] Begin play stop fire sound
  (Audio|Components|Audio|Stop (Variables|Default|GetFire%20Sound)))

(event EventMulticastDestroy
  ;[1 0 0] Multicast events
  ;;[1 1 1] Multicast destroy
  (|Destroy))

(event EventInteract
  (params (Player%20Component :type BP%20Player%20Inventory%20Component%20Object%20Reference))
  ;[0 1 0.09084] Server events
  ;;[1 1 1] Interact
  (|InteractEvents Player%20Component))

(event EventTarget
  ;[0 0.5089 1] Client events
  ;;[1 1 1] Player target
  (Rendering|SetRenderCustomDepth (Variables|Default|GetFurnace) true))

(event EventNotTarget
  ;[0 0.5089 1] Client events
  ;;[1 1 1] Not a player target
  (Rendering|SetRenderCustomDepth (Variables|Default|GetFurnace) false))

(event EventSwitchOffInteractAnimation
  ;[0 1 0.09084] Server events
  ;;[1 1 1] Switch off
  (|SwitchOffAnimation))

(event EventSwitchonInteractAnimation
  ;[0 1 0.09084] Server events
  ;;[1 1 1] Switch On
  (|SwitchOnAnimation))

(fn ConstructionScript)