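; BP_Blueprint is a holdable item, apparently a building plan, that gives the player input control over building.
; It forwards input to the PlayerBuildingComponent reached through the PlayerInventoryComponent.
; Holding the F input opens the build menu and releasing it closes it, while a left mouse press is passed on as a client-side build click.
; The construction script only calls the parent's.
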(event EventFInputAction
  (params (Key%20Down :type Boolean))
  (if Key%20Down
    (Default|ClientToggleBuildMenu (Variables|/Game/SurvivalGameKit/Blueprints/Components/BP_PlayerInventoryComponent.BP_PlayerInventoryComponent_C|GetPlayer%20Building%20Component (Variables|Default|GetPlayer%20Inventory%20Component)) true)
    (else
      (Default|ClientToggleBuildMenu (Variables|/Game/SurvivalGameKit/Blueprints/Components/BP_PlayerInventoryComponent.BP_PlayerInventoryComponent_C|GetPlayer%20Building%20Component (Variables|Default|GetPlayer%20Inventory%20Component)) false))))

(event EventLeftMouseInputAction
  (params (Key%20Down :type Boolean))
  (if Key%20Down
    (Default|ClientLeftMousePressed (Variables|/Game/SurvivalGameKit/Blueprints/Components/BP_PlayerInventoryComponent.BP_PlayerInventoryComponent_C|GetPlayer%20Building%20Component (Variables|Default|GetPlayer%20Inventory%20Component)))))

(fn ConstructionScript
  (|CallParentFunction))