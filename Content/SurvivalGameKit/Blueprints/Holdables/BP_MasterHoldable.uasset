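; Base Blueprint for holdable items that attach to the player character.
; On BeginPlay it snaps its AttachComponent to a named socket on the character mesh, reached through the player inventory component.
; A server-side Destroy event calls RemoveAllAttachmentsMessage before destroying the actor.
; Interaction functions return empty defaults and report the holdable as non-interactable.
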(event Custom|Destroy
  ;[0 1 0.09084] Server events
  ;;[1 1 1] Destroy this actor
  (Class|BPSurvivalInventoryInterface|RemoveAllAttachments(Message) self)
  (Actor|DestroyActor))

(event EventBeginPlay
  (Transformation|AttachComponentToComponent (Variables|Default|GetAttach%20Component) (Variables|/Script/Engine.Character|GetMesh (Variables|/Game/SurvivalGameKit/Blueprints/Components/BP_PlayerInventoryComponent.BP_PlayerInventoryComponent_C|GetMaster%20Character (Variables|NonEdit|GetPlayer%20Inventory%20Component))) (Variables|HoldableSettings|Socket|GetSocket%20Name) "SnapToTarget" "SnapToTarget" "SnapToTarget" true))

(fn ConstructionScript)

(fn InteractAction
  (return ""))

(fn InteractInputBrush
  (return ""))

(fn InteractName
  (return ""))

(fn InteractTime
  (return false 0.0))

(fn InteractingActionText
  (return ""))

(fn IsInteractable
  (return false))